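; First-person-style player character that handles look, movement and interaction through Enhanced Input, adding its mapping context and injecting its camera on BeginPlay.
; Look input is scaled by mouse speed and delta time, and both look and movement are blocked while interacting.
; Primary, cancel and alternative interactions call TryInteract with the camera, gated by blend state.
; Every Tick starts a walk or idle camera shake based on velocity.
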(event `self.ReceiveBeginPlay`
  ;[0 0 0 1 50] BeginPlay
  (`self.SetupInput`)
  (`self.InjectCamera` (`self.Camera`)))

(event `self.ReceiveTick`
  (params (DeltaSeconds :type "Float (single-precision)"))
  ;[0 0 0 1 30] Tick
  (`self.CameraShake`))

(event `EnhancedInput|/Game/Features/Player/Input/IA_CameraMove`
  (params (ActionValue :type "Vector2D Structure") (ElapsedSeconds :type "Float (double-precision)") (TriggeredSeconds :type "Float (double-precision)") (InputAction :type "InputAction Object Reference" :default "/Game/Features/Player/Input/IA_CameraMove.IA_CameraMove"))
  ;[0 0 0 1 32] Camera
  (:`Triggered`
    (if (not (`self.bIsInteracting`))
      (bind _calculatedvalue (`self.Calculate Mouse Movement` ActionValue_X))
      (`self.AddControllerYawInput` _calculatedvalue)
      (bind _calculatedvalue_2 (`self.Calculate Mouse Movement` ActionValue_Y true))
      (`self.AddControllerPitchInput` _calculatedvalue_2))))

(event `EnhancedInput|/Game/Features/Player/Input/IA_PlayerMovement`
  (params (ActionValue :type "Vector2D Structure") (ElapsedSeconds :type "Float (double-precision)") (TriggeredSeconds :type "Float (double-precision)") (InputAction :type "InputAction Object Reference" :default "/Game/Features/Player/Input/IA_PlayerMovement.IA_PlayerMovement"))
  (bind (_returnvalue_roll _returnvalue_pitch _returnvalue_yaw) (`KismetMathLibrary.BreakRotator` (`self.GetControlRotation`)))
  (bind (_returnvalue_roll_2 _returnvalue_pitch_2 _returnvalue_yaw_2) (`KismetMathLibrary.BreakRotator` (`self.GetControlRotation`)))
  ;[0 0 0 1 32] Movement
  (:`Triggered`
    (if (not (`self.bIsInteracting`))
      (`self.AddMovementInput` (`KismetMathLibrary.GetRightVector` (`KismetMathLibrary.MakeRotator` _returnvalue_roll 0.0 _returnvalue_yaw)) ActionValue_X)
      (`self.AddMovementInput` (`KismetMathLibrary.GetForwardVector` (`KismetMathLibrary.MakeRotator` 0.0 0.0 _returnvalue_yaw_2)) ActionValue_Y))))

(event `EnhancedInput|/Game/Features/Player/Input/IA_Interact`
  (params (ActionValue :type Boolean) (ElapsedSeconds :type "Float (double-precision)") (TriggeredSeconds :type "Float (double-precision)") (InputAction :type "InputAction Object Reference" :default "/Game/Features/Player/Input/IA_Interact.IA_Interact"))
  ;[0 0 0 1 32] Interaction handle
  (:`Triggered`
    (if (not (`self.bIsBlending`))
      (`self.TryInteract` (`self.Camera`)))))

(event `EnhancedInput|/Game/Features/Player/Input/IA_CancelInteraction`
  (params (ActionValue :type Boolean) (ElapsedSeconds :type "Float (double-precision)") (TriggeredSeconds :type "Float (double-precision)") (InputAction :type "InputAction Object Reference" :default "/Game/Features/Player/Input/IA_CancelInteraction.IA_CancelInteraction"))
  ;[0 0 0 1 32] Interaction handle
  (:`Triggered`
    (if (not (`self.bIsBlending`))
      (`self.TryInteract` (`self.Camera`) true))))

(event `EnhancedInput|/Game/Features/Player/Input/IA_SecondInteraction`
  (params (ActionValue :type Boolean) (ElapsedSeconds :type "Float (double-precision)") (TriggeredSeconds :type "Float (double-precision)") (InputAction :type "InputAction Object Reference" :default "/Game/Features/Player/Input/IA_SecondInteraction.IA_SecondInteraction"))
  ;[0 0 0 1 32] Interaction handle
  (:`Triggered`
    (if (`self.bIsBlending`)
      _
      (elif (not (`self.bIsInteracting`))
        (`self.TryInteract` (`self.Camera`) false true)))))

(fn `Calculate Mouse Movement`
  (params (value :type "Float (double-precision)") (invert :type Boolean))
  (returns (calculatedValue :type "Float (double-precision)"))
  (bind _returnvalue (* (* value (`GameplayStatics.GetWorldDeltaSeconds`)) (`self.MouseSpeed`)))
  (if invert
    (return (* _returnvalue -1.0))
    (else
      (return _returnvalue))))

(fn `CameraShake`
  (bind _returnvalue (`GameplayStatics.GetPlayerController` 0))
  (if (> (`KismetMathLibrary.VSize` (`self.GetVelocity`)) 0.0)
    (`PlayerController.ClientStartCameraShake` :`self` _returnvalue :`Shake` "/Game/Features/Player/CameraShake/CameraShakeWalk.CameraShakeWalk_C")
    (else
      (`PlayerController.ClientStartCameraShake` :`self` _returnvalue :`Shake` "/Game/Features/Player/CameraShake/CameraShakeIdle.CameraShakeIdle_C"))))

(fn `GetGameMode`
  (returns (NewParam :type "/Game/Levels/BP_SicilianGameModeBase Object Reference"))
  (bind _asbp_sicilian_game_mode_base (cast `/Game/Levels/BP_SicilianGameModeBase` (`GameplayStatics.GetGameMode`)))
  (return _asbp_sicilian_game_mode_base))

(fn `IsPlayerInteracting`)

(fn `SetupInput`
  (bind _asplayer_controller (cast `PlayerController` (`self.GetController`)))
  (bind _returnvalue (pcsubsystem `EnhancedInputLocalPlayerSubsystem` _asplayer_controller))
  (`/Engine/EditorBlueprintResources/StandardMacros.IsValid` _returnvalue
    (:`Is Valid`
      (`EnhancedInputSubsystemInterface.AddMappingContext` _returnvalue "/Game/Features/Player/Input/IM_Player.IM_Player" 0 (struct)))))

(fn `UserConstructionScript`)