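; BP_RequestActor is an actor that hosts the request and report widgets for the request feature.
; On BeginPlay it casts the Request and Raport component widgets to RequestWidget and hands each its RequestsManager reference.
; It then calls OnInject on each widget, a simple manual dependency injection.
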(event `self.ReceiveBeginPlay`
  (bind _requestsmanager (`self.RequestsManager`))
  (`|ExecutionSequence`
    (:`then_0`
      ;[1 1 1] Inject Request Manager
      (bind _asrequest_widget (cast `RequestWidget` (`WidgetComponent.GetWidget` (`self.Request`))))
      (set `RequestWidget.RequestManager` _requestsmanager _asrequest_widget)
      (`RequestWidget.OnInject` _asrequest_widget))
    (:`then_1`
      (bind _asrequest_widget_2 (cast `RequestWidget` (`WidgetComponent.GetWidget` (`self.Raport`))))
      (set `RequestWidget.RequestManager` _requestsmanager _asrequest_widget_2)
      (`RequestWidget.OnInject` _asrequest_widget_2))))

(fn `UserConstructionScript`)