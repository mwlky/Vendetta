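; Request manager that generates a request shortly after play begins and shows its text on the HUD.
; It caches the HUD manager and player character, then listens for the player's second interaction.
; During an active interaction, that input sends either the current request's letter or report text to the left panel, depending on whether the letter is open.
; Interaction start and finish events toggle the finished flag, with finish also disabling the HUD.
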(event `SetIsLetterOpened`
  (params (value :type Boolean))
  (set `self.IsLetterOpened` value))

(event `self.ReceiveBeginPlay`
  (`|ExecutionSequence`
    (:`then_0`
      ;[0 0 0 1 30] Init Request
      (`KismetSystemLibrary.Delay` 1.0)
      (`self.GenerateRequest`))
    (:`then_1`
      ;[0 0 0 1 40] Dependency
      (bind _asbp_hud_manager (cast `/Game/Features/UI/BP_HudManager` (`PlayerController.GetHUD` (`GameplayStatics.GetPlayerController` 0))))
      (set `self.HudManager` _asbp_hud_manager)
      (bind _asbp_player_character (cast `/Game/Features/Player/BP_PlayerCharacter` (`GameplayStatics.GetPlayerCharacter` 0)))
      (set `self.PlayerCharacter` _asbp_player_character))
    (:`then_2`
      ;[0 0 0 1 40] Panel Open
      (add `/Game/Features/Player/BP_PlayerCharacter.OnPlayerSecondInteraction` (`self.PlayerCharacter`) (delegate `OnPlayerSecondInteraction`)))
    (:`then_3`
      ;[0 0 0 1 40] Interaction Events
      (add `self.InteractionFinished` (delegate `InteractionFinished_Event`))
      (set `self.IsInteractionFinished` true :!label _label)
      (`/Game/Features/UI/BP_HudManager.Disable` (`self.HudManager`)))
    (:`then_4`
      (add `self.InteractionStarted` (delegate `InteractionStarted_Event`)))))

(event `OnPlayerSecondInteraction`
  (bind (_requestername _requestersurname _requesterdateofbirth _dateofarrest _letter _descriptiondata _nysid _topcharge _arrestid _crimedate _crimeage _type _reportdata) (break `Request` (`self.GetCurrentRequest`)))
  ;[0 0 0 1 40] Panel Open
  (if (`PlayerCharacter.bIsInteracting` (`self.PlayerCharacter`))
    (if (`self.IsInteractionFinished`)
      _
      (elif (`self.bIsLetterOpened`)
        (`/Game/Features/UI/BP_HudManager.HandleLeftTextPanel` (`self.HudManager`) (`.LetterText` (break `HandwrittenLetter` _letter)))
        (else
          (`/Game/Features/UI/BP_HudManager.HandleLeftTextPanel` (`self.HudManager`) (`.Text` (break `Report` _reportdata))))))))

(event `InteractionFinished_Event`
  ;[0 0 0 1 40] Interaction Events
  (goto _label))

(event `InteractionStarted_Event`
  ;[0 0 0 1 40] Interaction Events
  (set `self.IsInteractionFinished` false))

(fn `UserConstructionScript`)